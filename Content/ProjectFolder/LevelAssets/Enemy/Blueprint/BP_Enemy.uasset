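; BP_Enemy is an enemy that chases the player and deals damage on reaching them.
; After a short delay at BeginPlay, ChasePlayer runs AI MoveTo toward the player and re-calls itself on success or failure until EnemyDied is set.
; Arrival with CanAttack true clears the flag, starts RechargeAttack and calls DealDamage on Kenney_Main.
; RechargeAttack waits AttackRate but sets CanAttack false again, so nothing here re-enables attacking.
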(event `self.ReceiveBeginPlay`
  (`KismetSystemLibrary.Delay` 0.2)
  (`self.Chase Player`))

(event `Recharge Attack`
  (`KismetSystemLibrary.Delay` (`self.Attack Rate`))
  (set `self.Can Attack` false))

(event `Chase Player`
  (if (not (`self.Enemy Died`))
    (`|AIMoveTo` self (0.0 0.0 0.0) (`GameplayStatics.GetPlayerCharacter` 0)
      (:`OnSuccess`
        (if (`self.Can Attack`)
          (set `self.Can Attack` false)
          (`self.Recharge Attack`)
          (`self.Chase Player`)
          (bind _askenney_main (cast `/Game/ProjectFolder/Blueprints/Character/Kenney_Main` (`GameplayStatics.GetPlayerCharacter` 0)))
          (`/Game/ProjectFolder/Blueprints/Character/Kenney_Main.Deal Damage` _askenney_main (`self.Damage`))
          (else
            (`self.Chase Player` :!label _label))))
      (:`OnFail`
        (goto _label)))))

(fn `UserConstructionScript`)