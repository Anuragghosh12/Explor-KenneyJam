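; BP_Gate is a level-exit gate that sends the player to the Mortuary level once all collectables are gathered.
; Its Trigger overlap enables input on the gate when Kenney_Main enters and disables it on exit, so the F key only works nearby.
; Pressing F reads CollectableLeft from BP_Gacha1_GameMode and opens the level only when that count is zero.
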(event `Key|F`
  (params (Key :type "Key Structure"))
  (:`Pressed`
    (bind _asbp_gacha_1_game_mode (cast `/Game/ProjectFolder/Blueprints/BP_Gacha1_GameMode` (`GameplayStatics.GetGameMode`)))
    (bind _returnvalue (== (`/Game/ProjectFolder/Blueprints/BP_Gacha1_GameMode.Collectable Left` _asbp_gacha_1_game_mode) 0))
    (if _returnvalue
      (`GameplayStatics.OpenLevel` "Mortuary" _returnvalue))))

(event `self.Trigger.OnComponentBeginOverlap`
  (params (OverlappedComponent :type "PrimitiveComponent Object Reference") (OtherActor :type "Actor Object Reference") (OtherComp :type "PrimitiveComponent Object Reference") (OtherBodyIndex :type Integer) (bFromSweep :type Boolean) (SweepResult :type "HitResult Structure (by ref)"))
  (cast `/Game/ProjectFolder/Blueprints/Character/Kenney_Main` OtherActor)
  (`self.EnableInput` (`GameplayStatics.GetPlayerController` 0)))

(event `self.Trigger.OnComponentEndOverlap`
  (params (OverlappedComponent :type "PrimitiveComponent Object Reference") (OtherActor :type "Actor Object Reference") (OtherComp :type "PrimitiveComponent Object Reference") (OtherBodyIndex :type Integer))
  (cast `/Game/ProjectFolder/Blueprints/Character/Kenney_Main` OtherActor)
  (`self.DisableInput` (`GameplayStatics.GetPlayerController` 0)))

(fn `UserConstructionScript`)