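; Kenney_Main is a player character Blueprint that handles taking damage and dying.
; Its DealDamage event subtracts damage from Health.
; At zero or below, it shows the Death_Screen1 widget, disables input from the first player controller, then opens the TestingGrounds level after a short delay.
; BeginPlay, overlap and Tick are unused stubs, and the construction script only calls its parent.
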(event `Deal Damage`
  (params (Damage :type "Float (double-precision)"))
  (bind _output_get (set `self.Health` (- (`self.Health`) Damage)))
  (if (<= _output_get 0.0)
    (bind _returnvalue (`|GenericCreateObject` "/Game/Widget/Death_Screen1.Death_Screen1_C"))
    (`UserWidget.AddToViewport` _returnvalue 0)
    (`self.DisableInput` (`GameplayStatics.GetPlayerController` 0))
    (`KismetSystemLibrary.Delay` 1.0)
    (`GameplayStatics.OpenLevel` "TestingGrounds")))

(fn `UserConstructionScript`
  (`parent.UserConstructionScript`))